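; BP_ArenaBattleUnit is the visual actor for a battle unit in the arena, displaying states produced by simulation steps.
; BeginStateTransition stores the previous and new states, and Tick lerps position between their tile coordinates, converted to world space by BP_ArenaGameMode.
; When a transition ends, the unit hides itself if hit points are depleted, otherwise it snaps into place and scales HitPointsToken by remaining health fraction.
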(event `self.ReceiveBeginPlay`)

(event `self.ReceiveTick`
  (params (DeltaSeconds :type "Float (single-precision)"))
  (if (< (`self.StateTransitionElapsed`) (`self.StateTransitionDuration`))
    (bind _output_get (set `self.StateTransitionElapsed` (+ (`self.StateTransitionElapsed`) DeltaSeconds)))
    (if (>= _output_get (`self.StateTransitionDuration`))
      (`self.EndStateTransition`)
      (else
        (bind _asbp_arena_game_mode (cast `/Game/BP_ArenaGameMode` (`GameplayStatics.GetGameMode`)))
        (`self.K2_SetActorLocation` (`/Game/BP_ArenaGameMode.TileCoordinatesScaledWorldCoordinates` _asbp_arena_game_mode (`KismetMathLibrary.VLerp` (`.Coordinates` (break `ArenaBattleUnitState` (`self.FromState`))) (`.Coordinates` (break `ArenaBattleUnitState` (`self.ToState`))) (/ (`self.StateTransitionElapsed`) (`self.StateTransitionDuration`)))))))))

(fn `BeginStateTransition`
  (params (NewState :type "ArenaBattleUnitState Structure") (TransitionDuration :type "Float (double-precision)"))
  (set `self.FromState` (`self.ToState`))
  (set `self.ToState` NewState)
  (set `self.StateTransitionDuration` TransitionDuration)
  (set `self.StateTransitionElapsed` 0.0))

(fn `EndStateTransition`
  (bind (_teamlabel _coordinates _hitpoints _hitpointsmax) (break `ArenaBattleUnitState` (`self.ToState`)))
  (if (<= (`.HitPoints` (break `ArenaBattleUnitState` (`self.ToState`))) 0)
    ; We've died. Disappear!
    (`self.SetActorHiddenInGame` true)
    (else
      ; Update state to exactly match the target state.
      (bind _asbp_arena_game_mode (cast `/Game/BP_ArenaGameMode` (`GameplayStatics.GetGameMode`)))
      (`self.K2_SetActorLocation` (`/Game/BP_ArenaGameMode.TileCoordinatesScaledWorldCoordinates` _asbp_arena_game_mode (`.Coordinates` (break `ArenaBattleUnitState` (`self.ToState`)))))
      (`self.SetHitPointsTokenScale` (/ (`KismetMathLibrary.Conv_IntToDouble` _hitpoints) _hitpointsmax)))))

(fn `SetHitPointsTokenScale`
  (params (Scale :type "Float (double-precision)"))
  (`SceneComponent.SetRelativeScale3D` (`self.HitPointsToken`) (`KismetMathLibrary.Conv_DoubleToVector` Scale)))

(fn `UserConstructionScript`)