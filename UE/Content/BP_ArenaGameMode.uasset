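; Game mode that visualises an arena battle simulation by spawning and animating actors for its tiles and units.
; On battle begin it spawns hex or standard tiles per the simulation config and team-specific Blue or Red units at scaled tile coordinates.
; Each battle step ends every unit's current state transition and starts a new one toward its updated state over the step's delta time, matching units to states by array index.
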(event `self.OnBattleBegin`
  (params (Tiles :type "Array of ArenaBattleTile Structure (by ref)") (UnitStates :type "Array of ArenaBattleUnitState Structure (by ref)"))
  ; Render map tiles?
  (if true
    (`self.SpawnTiles` Tiles)
    (`self.SpawnUnitActors` UnitStates)))

(event `self.OnBattleStep`
  (params (DeltaSeconds :type "Float (single-precision)") (UnitStates :type "Array of ArenaBattleUnitState Structure (by ref)"))
  (for (_array_element _array_index) UnitStates
    (bind _output (`|GetArrayItem` (`self.UnitActors`) _array_index))
    (`/Game/BP_ArenaBattleUnit.EndStateTransition` _output)
    (`/Game/BP_ArenaBattleUnit.BeginStateTransition` _output _array_element DeltaSeconds)))

(fn `SpawnTiles`
  (params (Tiles :type "Array of ArenaBattleTile Structure"))
  (locals (NewLocalVar :type Boolean))
  (`KismetArrayLibrary.Array_Clear` (`self.TileActors`))
  (for _array_element Tiles
    (bind _returnvalue (`|SpawnActorFromClass` (select `bool` (`.bHexMap` (break `BattleSimulationConfig` (`self.BattleSimulationConfig`))) :`false` "/Game/BP_ArenaTile.BP_ArenaTile_C" :`true` "/Game/BP_ArenaHexTile.BP_ArenaHexTile_C" :!type "Actor Class Reference") (`KismetMathLibrary.MakeTransform` (`self.TileCoordinatesScaledWorldCoordinates` (`.Coordinates` (break `ArenaBattleTile` _array_element)))) "Undefined" "MultiplyWithRoot" null null))
    (`KismetArrayLibrary.Array_Add` (`self.TileActors`) _returnvalue)))

(fn `SpawnUnitActors`
  (params (SpawnStates :type "Array of ArenaBattleUnitState Structure"))
  (`KismetArrayLibrary.Array_Clear` (`self.UnitActors`))
  (for _array_element SpawnStates
    (bind (_teamlabel _coordinates) (break `ArenaBattleUnitState` _array_element))
    (bind _returnvalue (`|SpawnActorFromClass` (select `EBattleTeamLabel` _teamlabel :`Blue` "/Game/BP_ArenaBattleUnit_BlueTeam.BP_ArenaBattleUnit_BlueTeam_C" :`Red` "/Game/BP_ArenaBattleUnit_RedTeam.BP_ArenaBattleUnit_RedTeam_C" :!type "Actor Class Reference") (`KismetMathLibrary.MakeTransform` (`self.TileCoordinatesScaledWorldCoordinates` _coordinates)) "Undefined" "MultiplyWithRoot" null null))
    (bind _asbp_arena_battle_unit (cast `/Game/BP_ArenaBattleUnit` _returnvalue))
    (`KismetArrayLibrary.Array_Add` (`self.UnitActors`) _asbp_arena_battle_unit)
    (`/Game/BP_ArenaBattleUnit.BeginStateTransition` _asbp_arena_battle_unit _array_element 0.0)))

(fn `TileCoordinatesScaledWorldCoordinates`
  (params (WorldCoordinates :type "Vector Structure"))
  (returns (ScaledWorldCoordinates :type "Vector Structure"))
  (return (* (`self.TileCoordinatesToWorldCoordinates` WorldCoordinates) (`self.WorldScale`))))

(fn `UserConstructionScript`)